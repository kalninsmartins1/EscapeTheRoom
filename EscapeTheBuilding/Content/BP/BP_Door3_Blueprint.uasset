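; Swinging door Blueprint that opens and closes in response to events from its OpenDoor component.
; OnOpen plays the DoorSwing timeline, which adds a yaw angle to the rotation cached on BeginPlay, and OnClose reverses it.
; When the timeline finishes it notifies OpenDoor, playing the CloseDoor sound at the actor's location only after a close.
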(event `self.OpenDoor.OnOpen`
  (bind (_direction _door_open_angle) (`Timeline|Door swing` :!label _label)
    (:`Update`
      (`self.K2_SetActorRotation` (`KismetMathLibrary.ComposeRotators` (`KismetMathLibrary.MakeRotator` 0.0 0.0 _door_open_angle) (stale `self.ReceiveBeginPlay` _output_get))))
    (:`Finished`
      (`OpenDoor.OnDoorMovementFinished` (`self.OpenDoor`))
      (if (`self.ShouldPlayCloseSound`)
        (`GameplayStatics.PlaySoundAtLocation` "/Game/Audio/closeDoor.closeDoor" (`self.K2_GetActorLocation`))
        (set `self.ShouldPlayCloseSound` false)))))

(event `self.OpenDoor.OnClose`
  (set `self.ShouldPlayCloseSound` true)
  (goto _label :!via `Reverse`))

(event `self.ReceiveBeginPlay`
  (bind _output_get (set `self.InitialDoorRotation` (`self.K2_GetActorRotation`))))

(fn `UserConstructionScript`)